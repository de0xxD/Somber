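; PatrolRoute is a spline-based patrol path for enemies that tracks the current point along the route.
; IncrementPatrolRoute steps PatrolIndex by Direction and reverses Direction at the last and first spline points, giving a back-and-forth patrol.
; GetWorldSplinePosAsWorldPos returns the world-space location of the current point.
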(event `IncrementPatrolRoute`
  (bind _output_get (set `self.patrol index` (+ (`self.patrol index`) (`self.Direction`))))
  (if (== _output_get (- (`SplineComponent.GetNumberOfSplinePoints` (`self.PatrolRoute`)) 1))
    (set `self.Direction` -1)
    (elif (== (`self.patrol index`) 0)
      (set `self.Direction` 1))))

(fn `GetWorldSplinePos as World Pos`
  (returns (location :type "Vector Structure"))
  (return (`SplineComponent.GetLocationAtSplinePoint` (`self.PatrolRoute`) (`self.patrol index`) "World")))

(fn `UserConstructionScript`)