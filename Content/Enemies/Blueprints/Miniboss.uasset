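; Miniboss enemy Blueprint that fights with a cyber rocket launcher and keeps its damage component non-interruptible.
; EquipWeapon spawns the launcher, attaches it to the right-hand rifle socket and signals that equipping is done.
; Attack plays a fire montage whose Fire notify launches a rocket from the weapon toward the AI target's predicted position, leading it by distance-based travel time.
; Montage completion or interruption signals the attack's end.
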(event `/Game/Enemies/Blueprints/BPI_EnemyAI.EquipWeapon`
  (set `/Game/DamageSystem/BPC_DamageSystem.IsInterruptible` false (`self.BPC_DamageSystem`))
  (bind _returnvalue (`|SpawnActorFromClass` "/Game/Enemies/Weapons/BP_Weapon_CyberRocket.BP_Weapon_CyberRocket_C" (`KismetMathLibrary.MakeTransform` (0.0 0.0 0.0)) "Undefined" "MultiplyWithRoot" null null))
  (bind _output_get (set `self.WeaponActor` _returnvalue))
  (`self.K2_AttachToComponent` _output_get (`self.Mesh`) "Rifle_R" "KeepRelative" "KeepRelative" "KeepRelative" true)
  (`self.OnEquip`))

(event `/Game/Enemies/Blueprints/BPI_EnemyAI.Attack`
  (params (AttackTarget :type "Actor Object Reference"))
  (bind _returnvalue (`self.K2_GetActorLocation` (`self.WeaponActor`)))
  (`|PlayMontage` (`self.Mesh`) "/Game/Enemies/Blueprints/Anims/Cyber_Fire_Montage.Cyber_Fire_Montage" 0.8
    (:`then`
      (set `/Game/DamageSystem/BPC_DamageSystem.IsInterruptible` false (`self.BPC_DamageSystem`)))
    (:`OnCompleted`
      (`self.OnAttackEnd` :!label _label))
    (:`OnInterrupted`
      (goto _label))
    (:`OnNotifyBegin`
      (switch `name` "Fire"
        (:`Fire`
          (bind _asaic (cast `/Game/Enemies/Blueprints/AIC` (`AIBlueprintHelperLibrary.GetAIController` self)))
          (bind _attack_target (`/Game/Enemies/Blueprints/AIC.Attack Target` _asaic)
            (:`then`
              (bind _location (`self.CalculateFutureActorLocation` _attack_target (/ (`self.GetDistanceTo` _attack_target (`self.WeaponActor`)) 2500.0)))
              (`|SpawnActorFromClass` "/Game/Enemies/Weapons/BP_RocketLauncherProjectile.BP_RocketLauncherProjectile_C" (`KismetMathLibrary.MakeTransform` (+ _returnvalue (20.0 20.0 0.0)) (`KismetMathLibrary.FindLookAtRotation` _returnvalue _location)) "Undefined" "MultiplyWithRoot" null self)
              (`KismetSystemLibrary.Delay` 0.1)
              (set `/Game/DamageSystem/BPC_DamageSystem.IsInterruptible` false (`self.BPC_DamageSystem`)))
            (:`else`)))))))

(fn `UserConstructionScript`
  (`parent.UserConstructionScript`))