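; Melee enemy that spawns dual blades on its hand sockets and picks a short slash or long-range jump attack by target distance.
; Attacks reserve a token from the target, play a montage uninterruptible by damage, then return the token.
; Montage notifies drive forward sphere-trace damage against other teams, plus camera shake for the long-range slash.
; The jump launches along a suggested projectile arc toward the target's velocity-predicted position, stopping on landing.
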(event `/Game/Enemies/Blueprints/BPI_EnemyAI.EquipWeapon`
  (bind _returnvalue (`|SpawnActorFromClass` "/Game/Enemies/Weapons/BP_Weapon_Blade.BP_Weapon_Blade_C" (`self.GetTransform`) "Undefined" "MultiplyWithRoot" null null))
  (set `self.WeaponActor2` _returnvalue)
  (bind _returnvalue_2 (`|SpawnActorFromClass` "/Game/Enemies/Weapons/BP_Weapon_Blade.BP_Weapon_Blade_C" (`self.GetTransform`) "Undefined" "MultiplyWithRoot" null null))
  (set `self.WeaponActor` _returnvalue_2)
  (`self.K2_AttachToComponent` _returnvalue (`self.Mesh`) "Blade_R" "SnapToTarget" "SnapToTarget" "SnapToTarget" true)
  (`self.K2_AttachToComponent` _returnvalue_2 (`self.Mesh`) "Blade_L" "SnapToTarget" "SnapToTarget" "SnapToTarget" true)
  (set `self.IsWieldingWeapon` true)
  (`self.OnEquip`))

(event `self.ReceiveBeginPlay`
  (`self.EquipWeapon`)
  (`parent.ReceiveBeginPlay`))

(event `/Game/DamageSystem/BPI_Damageable.ReturnAttackToken`
  (params (Amount :type Integer))
  ;[1 1 1] Attacks
  (`parent.ReturnAttackToken` Amount))

(event `/Game/Enemies/Blueprints/BPI_EnemyAI.Attack`
  (params (AttackTarget :type "Actor Object Reference"))
  (bind _returnvalue (`KismetMathLibrary.Vector_Distance` (`self.K2_GetActorLocation` AttackTarget) (`self.K2_GetActorLocation` self)))
  ;[1 1 1] Attacks
  (if (and (>= _returnvalue 401.0) (<= _returnvalue 900.0))
    (`self.LongRangeAttack` AttackTarget)
    (elif (<= _returnvalue 400.0)
      (`self.ShortRangeAttack` AttackTarget))))

(event `SphereTraceDamage`
  (params (Damage :type "Float (double-precision)" :default 25.0) (Radius :type "Float (double-precision)" :default 30.0) (DamageResponse :type "/Game/DamageSystem/E_DamageResponse Enum" :default "NewEnumerator0"))
  (bind _returnvalue (`self.K2_GetActorLocation`))
  ;[1 1 1] AttackHelper
  (bind _outhit (`KismetSystemLibrary.SphereTraceSingleForObjects` _returnvalue (+ _returnvalue (* (`self.GetActorForwardVector`) 210.0)) Radius (`|MakeArray` "ObjectTypeQuery3" :!type "EObjectTypeQuery Enum")))
  (if true
    (bind (_bblockinghit _binitialoverlap _time _distance _location _impactpoint _normal _impactnormal _physmat _hitactor) (`GameplayStatics.BreakHitResult` _outhit))
    (bind _teamnumber (message `/Game/DamageSystem/BPI_Damageable.GetTeamNumber` _hitactor))
    (if (!= (`self.Team Number`) _teamnumber)
      (message `/Game/DamageSystem/BPI_Damageable.TakeDamage` _hitactor (make `/Game/DamageSystem/S_DamageInfo` Damage "NewEnumerator1" DamageResponse) self))))

(event `ShortRangeAttack`
  (params (AttackTarget :type "Actor Object Reference"))
  ;[1 1 1] Attacks
  (`parent.Attack` AttackTarget)
  (bind _succes (message `/Game/DamageSystem/BPI_Damageable.ReserveAttackToken` AttackTarget 1))
  (if _succes
    (bind _notifyname (`|PlayMontage` (`self.Mesh`) "/Game/Enemies/Blueprints/Anims/Attack_Montage.Attack_Montage")
      (:`then`
        (set `/Game/DamageSystem/BPC_DamageSystem.IsInterruptible` false (`self.BPC_DamageSystem`)))
      (:`OnCompleted`
        (`self.OnAttackEnd` :!label _label)
        (message `/Game/DamageSystem/BPI_Damageable.ReturnAttackToken` AttackTarget 1)
        (set `/Game/DamageSystem/BPC_DamageSystem.IsInterruptible` true (`self.BPC_DamageSystem`)))
      (:`OnInterrupted`
        (goto _label))
      (:`OnNotifyBegin`
        (switch `name` _notifyname
          (:`Slash`
            (`self.SphereTraceDamage` 45.0 30.0 "NewEnumerator1")))))
    (else
      (`KismetSystemLibrary.DelayUntilNextTick`)
      (`self.OnAttackEnd`))))

(event `LongRangeAttack`
  (params (AttackTarget :type "Actor Object Reference"))
  ;[1 1 1] Attacks
  (`parent.Attack` AttackTarget)
  (bind _succes (message `/Game/DamageSystem/BPI_Damageable.ReserveAttackToken` AttackTarget 1))
  (if _succes
    (bind _notifyname (`|PlayMontage` (`self.Mesh`) "/Game/Enemies/Blueprints/Anims/JumpAttack_Montage.JumpAttack_Montage")
      (:`then`
        (set `/Game/DamageSystem/BPC_DamageSystem.IsInterruptible` false (`self.BPC_DamageSystem`)))
      (:`OnCompleted`
        (`self.OnAttackEnd` :!label _label_2)
        (message `/Game/DamageSystem/BPI_Damageable.ReturnAttackToken` AttackTarget 1)
        (set `/Game/DamageSystem/BPC_DamageSystem.IsInterruptible` true (`self.BPC_DamageSystem`)))
      (:`OnInterrupted`
        (goto _label_2))
      (:`OnNotifyBegin`
        (switch `name` _notifyname
          (:`Slash`
            (`self.SphereTraceDamage` 30.0 190.0 "NewEnumerator2")
            (`GameplayStatics.PlayWorldCameraShake` "/Game/Character/CamEffects/BP_Melee_Longrange.BP_Melee_Longrange_C" (`self.K2_GetActorLocation`) 300.0 700.0 1.2 true))
          (:`Jump`
            (`self.JumpToAttackTarget` AttackTarget)))))
    (else
      (`KismetSystemLibrary.DelayUntilNextTick`)
      (`self.OnAttackEnd`))))

(event `JumpToAttackTarget`
  (params (AttackTarget :type "Actor Object Reference"))
  ;[1 1 1] AttackHelper
  (bind _location (`self.CalculateFutureActorLocation` AttackTarget 0.5))
  (bind _outlaunchvelocity (`GameplayStatics.SuggestProjectileVelocity_CustomArc` (`self.K2_GetActorLocation`) (`KismetMathLibrary.MakeVector` (.x _location) (.y _location) (+ (.z _location) 100.0))))
  (`self.LaunchCharacter` (`KismetMathLibrary.MakeVector` (.x _outlaunchvelocity) (.y _outlaunchvelocity) (- (.z _outlaunchvelocity) 400.0)))
  (add `self.LandedDelegate` (delegate `OnLand`)))

(event `self.Death`
  ;[1 1 1] Attacks
  (`parent.Death`))

(event `OnLand` :!signature `self.LandedDelegate`
  (params (Hit :type "HitResult Structure (by ref)"))
  ;[1 1 1] AttackHelper
  (remove `self.LandedDelegate` (delegate `OnLand`))
  (`MovementComponent.StopMovementImmediately` (`self.CharacterMovement`)))

(fn `AttackStart`
  (params (AttackTarget :type "Actor Object Reference") (TokensNeeded :type Integer))
  (returns (Success :type Boolean))
  (return false))

(fn `CalculateFutureActorLocation`
  (params (Actor :type "Actor Object Reference") (Time :type "Float (double-precision)" :default 1.0))
  (returns (Location :type "Vector Structure"))
  (return (+ (`self.K2_GetActorLocation` Actor) (* (* (`self.GetVelocity` Actor) (1.0 1.0 1.0)) Time))))

(fn `SetMovementSpeed`
  (params (Speed :type "/Game/Enemies/Blueprints/Enums/E_MovementSpeed Enum" :default "NewEnumerator0"))
  (returns (SpeedValue :type "Float (double-precision)"))
  (bind _output_get (set `CharacterMovementComponent.MaxWalkSpeed` (select `/Game/Enemies/Blueprints/Enums/E_MovementSpeed` Speed :`NewEnumerator1` 130.0 :`NewEnumerator2` 700.0 :`NewEnumerator3` 1400.0 :!type "Float (single-precision)") (`self.CharacterMovement`)))
  (return _output_get))

(fn `UserConstructionScript`
  (bind _bpc_damagesystem (`self.BPC_DamageSystem`))
  (bind _output_get (set `/Game/DamageSystem/BPC_DamageSystem.MaxHealth` 200.0 _bpc_damagesystem))
  (set `/Game/DamageSystem/BPC_DamageSystem.Health` _output_get _bpc_damagesystem)
  (`parent.UserConstructionScript`))