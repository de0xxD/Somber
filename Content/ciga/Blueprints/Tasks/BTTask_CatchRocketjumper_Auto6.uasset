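; Behavior tree task that sends the AI after the player while they are airborne, apparently to catch rocket jumpers.
; On execute, if player 0's character movement is falling, it issues a move to that character's last update X and Y at a fixed height with a tight acceptance radius.
; The task finishes successfully at once, without waiting for the move to complete.
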(event `self.ReceiveExecuteAI`
  (params (OwnerController :type "AIController Object Reference") (ControlledPawn :type "Pawn Object Reference"))
  (bind _returnvalue (`GameplayStatics.GetPlayerCharacter` 0))
  (if (`NavMovementComponent.IsFalling` (`Character.CharacterMovement` _returnvalue))
    (`AIController.MoveToLocation` OwnerController (+ (`KismetMathLibrary.MakeVector` (.x (`CharacterMovementComponent.GetLastUpdateLocation` (`Character.CharacterMovement` _returnvalue))) (.y (`CharacterMovementComponent.GetLastUpdateLocation` (`Character.CharacterMovement` _returnvalue)))) (0.0 0.0 195.15)) 20.0 true true false true null true))
  (`self.FinishExecute` true))