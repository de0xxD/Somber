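; Base enemy character that wraps a damage component behind damage, healing, team, patrol and movement-speed functions for its AI controller and other actors.
; Hits freeze the AI and play a reaction montage, then resume attacking the damage causer and show the health bar, unless the player is falling.
; Death ragdolls the mesh, stops AI logic, plays effects and returns stored attack tokens to their owners.
; Jumps use suggested projectile-arc launch velocities.
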(event `self.ReceiveBeginPlay`
  (bind _bpc_damagesystem (`self.BPC_DamageSystem`))
  (bind _asaic (cast `/Game/Enemies/Blueprints/AIC` (`AIBlueprintHelperLibrary.GetAIController` self)))
  (set `self.AIController` _asaic)
  (bind _returnvalue (`|CreateWidget` "/Game/DamageSystem/W_HealthBar.W_HealthBar_C" null self))
  (`WidgetComponent.SetWidget` (`self.HealthBar`) _returnvalue)
  (add `/Game/DamageSystem/BPC_DamageSystem.OnDeath` _bpc_damagesystem (`|CreateDelegate` :!event `Death`))
  (add `/Game/DamageSystem/BPC_DamageSystem.OnDamageResponse` _bpc_damagesystem (`|CreateDelegate` :!event `HitResponse`)))

(event `Death`
  (bind _mesh (`self.Mesh`))
  (`PrimitiveComponent.SetSimulatePhysics` _mesh true)
  (`PrimitiveComponent.SetCollisionEnabled` _mesh "QueryAndPhysics")
  (`BrainComponent.StopLogic` (`AIController.BrainComponent` (`self.AIController`)) "")
  (`ActorComponent.K2_DestroyComponent` (`self.HealthBar`))
  (`GameplayStatics.PlaySoundAtLocation` "/Game/Sounds/Enemies/14__Serious_Sam_-_Sound_Effects_-_Bio_Mechanoid__mp3cut_net_.14__Serious_Sam_-_Sound_Effects_-_Bio_Mechanoid__mp3cut_net_" (`self.K2_GetActorLocation`) (struct) 0.5 0.9 0.0 null null null null)
  (`/Game/Enemies/Blueprints/AIC.SetStateAsDead` (`self.AIController`))
  (bind _returnvalue (`GameplayStatics.SpawnEmitterAttached` "/Game/StarterContent/Particles/P_Sparks.P_Sparks" (`self.Mesh`) "Head" (0.0 0.0 0.0) (struct) (2.0 2.0 2.0)))
  (`ActorComponent.K2_DestroyComponent` (`self.CapsuleComponent`))
  (`KismetSystemLibrary.Delay` 1.5)
  (`ActorComponent.K2_DestroyComponent` _returnvalue)
  (bind _keys (`BlueprintMapLibrary.Map_Keys` (`self.ReservedAttackTokens`)))
  (for _array_element _keys
    (message `/Game/DamageSystem/BPI_Damageable.ReturnAttackToken` _array_element (`BlueprintMapLibrary.Map_Find` (`self.ReservedAttackTokens`) _array_element))))

(event `HitResponse`
  (params (DamageResponse :type "/Game/DamageSystem/E_DamageResponse Enum" :default "NewEnumerator0") (DamageCauser :type "Actor Object Reference"))
  (`MovementComponent.StopMovementImmediately` (`self.CharacterMovement`))
  (`/Game/Enemies/Blueprints/AIC.SetStateAsFrozen` (`self.AIController`))
  (`|PlayMontage` (`self.Mesh`) (`self.HitReactionMontage`) 2.0 0.5
    (:`OnCompleted`
      _)
    (:`OnInterrupted`
      _))
  (if (not (`NavMovementComponent.IsFalling` (`self.GetMovementComponent` (`GameplayStatics.GetPlayerCharacter` 0))))
    (`/Game/Enemies/Blueprints/AIC.SetStateAsAttacking` (`self.AIController`) DamageCauser true)
    (`SceneComponent.SetVisibility` (`self.HealthBar`) true false)))

(event `/Game/Enemies/Blueprints/BPI_EnemyAI.JumpToDestination`
  (params (Destination :type "Vector Structure"))
  (bind _outlaunchvelocity (`GameplayStatics.SuggestProjectileVelocity_CustomArc` (`self.K2_GetActorLocation`) (`KismetMathLibrary.MakeVector` (.x Destination) (.y Destination) (+ (.z Destination) 250.0))))
  (`self.LaunchCharacter` _outlaunchvelocity true))

(event `/Game/DamageSystem/BPI_Damageable.ReturnAttackToken`
  (params (Amount :type Integer))
  (`/Game/DamageSystem/BPC_DamageSystem.ReturnAttackToken` (`self.BPC_DamageSystem`) Amount))

(event `/Game/Enemies/Blueprints/BPI_EnemyAI.Attack`
  (params (AttackTarget :type "Actor Object Reference"))
  (set `self.Attacking` true))

(event `/Game/Enemies/Blueprints/BPI_EnemyAI.StoreAttackTokens`
  (params (Actor :type "Actor Object Reference") (Amount :type Integer))
  (bind (_value _returnvalue) (`BlueprintMapLibrary.Map_Find` (`self.ReservedAttackTokens`) Actor))
  (`BlueprintMapLibrary.Map_Add` (`self.ReservedAttackTokens`) Actor (`KismetMathLibrary.SelectInt` (+ _value Amount) Amount _returnvalue)))

(fn `CanSenseActor`
  (returns (Actor :type "Actor Object Reference") (Sense :type "Actor Object Reference"))
  (return null null))

(fn `GetCurrentHealth`
  (returns (Health :type "Float (double-precision)"))
  (return (`/Game/DamageSystem/BPC_DamageSystem.Health` (`self.BPC_DamageSystem`))))

(fn `GetIdealRange`
  (returns (AttackRadius :type "Float (double-precision)") (DefendRadius :type "Float (double-precision)"))
  (return 2000.0 2000.0))

(fn `GetMaxHealth`
  (returns (MaxHealth :type "Float (double-precision)"))
  (return (`/Game/DamageSystem/BPC_DamageSystem.MaxHealth` (`self.BPC_DamageSystem`))))

(fn `GetPatrolRoute`
  (returns (PatrolRoute :type "/Game/Enemies/Blueprints/PatrolRoute Object Reference"))
  (return (`self.PatrolRoute`)))

(fn `GetTeamNumber`
  (returns (TeamNumber :type Integer))
  (return (`self.Team Number`)))

(fn `Heal`
  (params (Amount :type "Float (double-precision)"))
  (returns (NewHealth :type "Float (double-precision)"))
  (bind _newhealth (`/Game/DamageSystem/BPC_DamageSystem.Heal` (`self.BPC_DamageSystem`) Amount))
  (return _newhealth))

(fn `IsDead`
  (returns (Dead :type Boolean))
  (return (`/Game/DamageSystem/BPC_DamageSystem.IsDead` (`self.BPC_DamageSystem`))))

(fn `ReserveAttackToken`
  (params (Amount :type Integer))
  (returns (Succes :type Boolean))
  (bind _success (`/Game/DamageSystem/BPC_DamageSystem.ReserveAttackToken` (`self.BPC_DamageSystem`) Amount))
  (return _success))

(fn `SetMovementSpeed`
  (params (Speed :type "/Game/Enemies/Blueprints/Enums/E_MovementSpeed Enum" :default "NewEnumerator0"))
  (returns (SpeedValue :type "Float (double-precision)"))
  (bind _output_get (set `CharacterMovementComponent.MaxWalkSpeed` (select `/Game/Enemies/Blueprints/Enums/E_MovementSpeed` Speed :`NewEnumerator1` 120.0 :`NewEnumerator2` 800.0 :`NewEnumerator3` 1600.0 :!type "Float (single-precision)") (`self.CharacterMovement`)))
  (return _output_get))

(fn `TakeDamage`
  (params (DamageInfo :type "/Game/DamageSystem/S_DamageInfo Structure") (DamageCauser :type "Actor Object Reference"))
  (returns (WasDamaged :type Boolean))
  (bind _wasdamaged (`/Game/DamageSystem/BPC_DamageSystem.Take Damage` (`self.BPC_DamageSystem`) DamageInfo DamageCauser))
  (return _wasdamaged))

(fn `UserConstructionScript`)