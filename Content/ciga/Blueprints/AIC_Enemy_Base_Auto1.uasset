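; AI controller for enemies that runs a behavior tree and manages a passive or attacking state.
; On possess it starts the Drevo behavior tree and sets the state to passive.
; Two functions write the E_AI_States enum to the Blackboard, and the attacking one also stores the attack target object.
; Nothing in this controller calls the attacking switch.
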(event `self.ReceivePossess`
  (params (PossessedPawn :type "Pawn Object Reference"))
  (`self.RunBehaviorTree` "/Game/Enemies/Blueprints/Drevo.Drevo")
  (`self.SetStateAsPassive`))

(fn `SetStateAsAttacking`
  (params (AttackTarget :type "Actor Object Reference"))
  (`BlackboardComponent.SetValueAsObject` (`self.Blackboard`) (`self.Attack Target Key Name`) AttackTarget)
  (`BlackboardComponent.SetValueAsEnum` (`self.Blackboard`) (`self.StateKeyName`) (enumliteral `/Game/Enemies/Blueprints/Enums/E_AI_States` "NewEnumerator1")))

(fn `SetStateAsPassive`
  (`BlackboardComponent.SetValueAsEnum` (`self.Blackboard`) (`self.StateKeyName`) (enumliteral `/Game/Enemies/Blueprints/Enums/E_AI_States` "NewEnumerator0")))

(fn `UserConstructionScript`)