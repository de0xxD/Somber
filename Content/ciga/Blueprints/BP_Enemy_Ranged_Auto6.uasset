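; BP_Enemy_Ranged_Auto6 is a rifle-wielding ranged enemy that extends a parent enemy class.
; On BeginPlay it attaches a rifle to its hand socket, and it overrides movement speeds and long ideal ranges.
; Attack plays a fire montage whose notify spawns a projectile near the capsule, using capsule rotation, when the AI controller has a valid target.
; A debug line trace to the target runs first, but its result does not affect firing.
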(event `self.ReceiveBeginPlay`
  (`/Game/Enemies/Blueprints/BPI_EnemyAI.EquipWeapon`)
  (`parent.ReceiveBeginPlay`))

(event `/Game/Enemies/Blueprints/BPI_EnemyAI.EquipWeapon`
  (bind _returnvalue (`|SpawnActorFromClass` "/Game/Enemies/Weapons/BP_Weapon_Rifle.BP_Weapon_Rifle_C" (`KismetMathLibrary.MakeTransform` (0.0 0.0 0.0)) "Undefined" "MultiplyWithRoot" null null))
  (bind _output_get (set `self.WeaponActor` _returnvalue))
  (`self.K2_AttachToComponent` _output_get (`self.Mesh`) "Rifle_R" "KeepRelative" "KeepRelative" "KeepRelative" true)
  (`self.OnEquip`))

(event `/Game/Enemies/Blueprints/BPI_EnemyAI.Attack`
  (bind _capsulecomponent (`self.CapsuleComponent`))
  (bind _notifyname (`|PlayMontage` (`self.Mesh`) "/Game/Enemies/Blueprints/Anims/Fire_Montage.Fire_Montage")
    (:`OnCompleted`
      (`self.OnAttackEnd` :!label _label))
    (:`OnInterrupted`
      (goto _label))
    (:`OnNotifyBegin`
      (switch `name` _notifyname
        (:`Fire`
          (bind _asaic (cast `/Game/Enemies/Blueprints/AIC` (`AIBlueprintHelperLibrary.GetAIController` self)))
          (bind _attack_target (`/Game/Enemies/Blueprints/AIC.Attack Target` _asaic)
            (:`then`
              (bind (_outhit _returnvalue) (`KismetSystemLibrary.LineTraceSingle` :`Start` (`self.K2_GetActorLocation` (`self.WeaponActor`)) :`End` (`self.K2_GetActorLocation` _attack_target) :`TraceChannel` "TraceTypeQuery1" :`DrawDebugType` "ForDuration"))
              (if _returnvalue
                _
                (else
                  _))
              (`|SpawnActorFromClass` "/Game/Enemies/Weapons/BP_Projectile.BP_Projectile_C" (`KismetMathLibrary.MakeTransform` (+ (`SceneComponent.K2_GetComponentLocation` _capsulecomponent) (0.0 70.0 40.0)) (`SceneComponent.K2_GetComponentRotation` _capsulecomponent)) "Undefined" "MultiplyWithRoot" null self))
            (:`else`)))))))

(fn `GetIdealRange`
  (returns (AttackRadius :type "Float (double-precision)") (DefendRadius :type "Float (double-precision)"))
  (return 2000.0 2000.0))

(fn `SetMovementSpeed`
  (params (Speed :type "/Game/Enemies/Blueprints/Enums/E_MovementSpeed Enum" :default "NewEnumerator0"))
  (returns (SpeedValue :type "Float (double-precision)"))
  (bind _output_get (set `CharacterMovementComponent.MaxWalkSpeed` (select `/Game/Enemies/Blueprints/Enums/E_MovementSpeed` Speed :`NewEnumerator1` 90.0 :`NewEnumerator2` 600.0 :`NewEnumerator3` 800.0 :!type "Float (single-precision)") (`self.CharacterMovement`)))
  (return _output_get))

(fn `UserConstructionScript`
  (`parent.UserConstructionScript`))