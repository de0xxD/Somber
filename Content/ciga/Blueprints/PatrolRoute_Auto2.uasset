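; Patrol route Blueprint built on a PatrolRoute spline, exposing the world position of the current route point.
; GetWorldSplinePosAsWorldPos returns the spline point location at PatrolIndex.
; IncrementPatrolRoute is an empty event, so nothing here advances the index.
; Disconnected logic sketches a ping-pong Direction flip at the route ends, but it never runs and its index sum is unused.
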(event `IncrementPatrolRoute`)

(fn `GetWorldSplinePos as World Pos`
  (returns (location :type "Vector Structure"))
  (return (`SplineComponent.GetLocationAtSplinePoint` (`self.PatrolRoute`) (`self.patrol index`) "World")))

(fn `UserConstructionScript`)