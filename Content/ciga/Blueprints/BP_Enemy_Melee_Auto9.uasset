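; BP_Enemy_Melee_Auto9 is a melee enemy character that dual-wields blades.
; On BeginPlay it spawns two BP_Blade actors and snaps them to the Blade_L and Blade_R sockets on its mesh.
; Its Attack event plays an attack montage and fires OnAttackEnd whether the montage completes or is interrupted.
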(event `self.ReceiveBeginPlay`
  (`self.WieldBlade`))

(event `/Game/Enemies/Blueprints/BPI_EnemyAI.Attack`
  (`|PlayMontage` (`self.Mesh`) "/Game/Enemies/Enemy_Bot/Attack_Montage.Attack_Montage"
    (:`OnCompleted`
      _)
    (:`OnInterrupted`
      _))
  (`self.OnAttackEnd`))

(event `WieldBlade`
  (bind _mesh (`self.Mesh`))
  (bind _returnvalue (`|SpawnActorFromClass` "/Game/Enemies/Blueprints/Weapons/BP_Blade.BP_Blade_C" (`self.GetTransform`) "Undefined" "MultiplyWithRoot" null null))
  (`self.K2_AttachToComponent` _returnvalue _mesh "Blade_L" "SnapToTarget" "SnapToTarget" "SnapToTarget" true)
  (bind _returnvalue_2 (`|SpawnActorFromClass` "/Game/Enemies/Blueprints/Weapons/BP_Blade.BP_Blade_C" (`self.GetTransform`) "Undefined" "MultiplyWithRoot" null null))
  (`self.K2_AttachToComponent` _returnvalue_2 _mesh "Blade_R" "SnapToTarget" "SnapToTarget" "SnapToTarget" true))

(fn `NewFunction`)

(fn `UserConstructionScript`
  (`parent.UserConstructionScript`))