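; Melee enemy child Blueprint that dual-wields blades, setting its own health and walk speed for each movement state.
; On BeginPlay it spawns two blade actors on hand sockets before running parent logic.
; Attack plays a montage, blocking interruption through the damage system until it completes or is interrupted, then signals attack end.
; A montage notify triggers a short forward sphere trace against pawns to deal damage.
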(event `self.ReceiveBeginPlay`
  (`self.EquipWeapon`)
  (`parent.ReceiveBeginPlay`))

(event `/Game/Enemies/Blueprints/BPI_EnemyAI.Attack`
  (bind _returnvalue (`self.K2_GetActorLocation`))
  (bind _notifyname (`|PlayMontage` (`self.Mesh`) "/Game/Enemies/Blueprints/Anims/Attack_Montage.Attack_Montage")
    (:`then`
      (set `/Game/DamageSystem/BPC_DamageSystem.IsInterruptible` false (`self.BPC_DamageSystem`)))
    (:`OnCompleted`
      (`self.OnAttackEnd` :!label _label)
      (set `/Game/DamageSystem/BPC_DamageSystem.IsInterruptible` true (`self.BPC_DamageSystem`)))
    (:`OnInterrupted`
      (goto _label))
    (:`OnNotifyBegin`
      (switch `name` _notifyname
        (:`Slash`
          (bind _outhit (`KismetSystemLibrary.SphereTraceSingleForObjects` :`Start` _returnvalue :`End` (+ _returnvalue (* (`self.GetActorForwardVector`) 200.0)) :`Radius` 30.0 :`ObjectTypes` (`|MakeArray` "ObjectTypeQuery3" :!type "EObjectTypeQuery Enum") :`DrawDebugType` "ForDuration"))
          (if true
            (message `/Game/DamageSystem/BPI_Damageable.TakeDamage` (`.HitActor` (`GameplayStatics.BreakHitResult` _outhit)) (make `/Game/DamageSystem/S_DamageInfo` 25.0 "NewEnumerator1"))))))))

(event `/Game/Enemies/Blueprints/BPI_EnemyAI.EquipWeapon`
  (bind _returnvalue (`|SpawnActorFromClass` "/Game/Enemies/Weapons/BP_Weapon_Blade.BP_Weapon_Blade_C" (`self.GetTransform`) "Undefined" "MultiplyWithRoot" null null))
  (bind _returnvalue_2 (`|SpawnActorFromClass` "/Game/Enemies/Weapons/BP_Weapon_Blade.BP_Weapon_Blade_C" (`self.GetTransform`) "Undefined" "MultiplyWithRoot" null null))
  (set `self.WeaponActor` _returnvalue_2)
  (`self.K2_AttachToComponent` _returnvalue (`self.Mesh`) "Blade_R" "SnapToTarget" "SnapToTarget" "SnapToTarget" true)
  (`self.K2_AttachToComponent` _returnvalue_2 (`self.Mesh`) "Blade_L" "SnapToTarget" "SnapToTarget" "SnapToTarget" true)
  (set `self.IsWieldingWeapon` true)
  (`self.OnEquip`))

(fn `SetMovementSpeed`
  (params (Speed :type "/Game/Enemies/Blueprints/Enums/E_MovementSpeed Enum" :default "NewEnumerator0"))
  (returns (SpeedValue :type "Float (double-precision)"))
  (bind _output_get (set `CharacterMovementComponent.MaxWalkSpeed` (select `/Game/Enemies/Blueprints/Enums/E_MovementSpeed` Speed :`NewEnumerator1` 130.0 :`NewEnumerator2` 700.0 :`NewEnumerator3` 1400.0 :!type "Float (single-precision)") (`self.CharacterMovement`)))
  (return _output_get))

(fn `UserConstructionScript`
  (bind _bpc_damagesystem (`self.BPC_DamageSystem`))
  (bind _output_get (set `/Game/DamageSystem/BPC_DamageSystem.MaxHealth` 200.0 _bpc_damagesystem))
  (set `/Game/DamageSystem/BPC_DamageSystem.Health` _output_get _bpc_damagesystem)
  (`parent.UserConstructionScript`))